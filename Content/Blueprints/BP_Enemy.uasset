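; Enemy actor that loses health when its cube is hit by Projectile-tagged components and destroys itself when health reaches exactly zero.
; Tick copies the game mode's Start value and refreshes NewLocation from the Target's sprite, as BeginPlay and construction also do.
; Within range of that location it starts a looping crocodile attack animation once.
; No movement logic is present; the IsArived branch is empty and a ripple emitter is unconnected.
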(event `self.Cube.OnComponentHit`
  (params (HitComponent :type "PrimitiveComponent Object Reference") (OtherActor :type "Actor Object Reference") (OtherComp :type "PrimitiveComponent Object Reference") (NormalImpulse :type "Vector Structure") (Hit :type "HitResult Structure (by ref)"))
  (if (`ActorComponent.ComponentHasTag` OtherComp "Projectile")
    (set `self.Health` (- (`self.Health`) 100.0))))

(event `self.ReceiveTick`
  (params (DeltaSeconds :type "Float (single-precision)"))
  (`|ExecutionSequence`
    (:`then_0`
      (if (== (`self.Health`) 0.0)
        (`/Engine/EditorBlueprintResources/StandardMacros.DoOnce` false
          (:`Completed`
            (`self.K2_DestroyActor` self)))))
    (:`then_1`
      (if (== (`self.K2_GetActorLocation` self) (`self.NewLocation`) :`ErrorTolerance` 70.0)
        (`/Engine/EditorBlueprintResources/StandardMacros.DoOnce` false
          (:`Completed`
            (`SkeletalMeshComponent.PlayAnimation` (`self.SkeletalMesh`) "/Game/Animations/A_CrocoAttacke.A_CrocoAttacke" true)))))
    (:`then_2`
      (if (not (`self.IsArived`))
        _))
    (:`then_3`
      (bind _asbp_game_mode (cast `/Game/Blueprints/BP_GameMode` (`GameplayStatics.GetGameMode`)))
      (set `self.Start` (`/Game/Blueprints/BP_GameMode.Start` _asbp_game_mode)))
    (:`then_4`
      (set `self.NewLocation` (`SceneComponent.K2_GetComponentLocation` (`TargetPoint.SpriteComponent` (`self.Target`))) :!label _label))))

(event `self.ReceiveBeginPlay`
  (goto _label))

(fn `UserConstructionScript`
  (set `self.NewLocation` (`SceneComponent.K2_GetComponentLocation` (`TargetPoint.SpriteComponent` (`self.Target`)))))