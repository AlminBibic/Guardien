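; BP_GameMode is a game mode that runs an end countdown while the Eggs count equals five.
; Tick creates and adds a WBP_Timer widget on every qualifying frame, with no guard against duplicates.
; A one-second Delay on the same Tick paces the decrement of Seconds, which rolls over into Minutes.
; When both reach zero, a DoOnce prints "GameOver".
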(event `self.ReceiveTick`
  (params (DeltaSeconds :type "Float (single-precision)"))
  (`|ExecutionSequence`
    (:`then_0`
      (if (== (`self.eggs`) 5)
        (bind _returnvalue (`|CreateWidget` "/Game/Blueprints/WBP_Timer.WBP_Timer_C"))
        (`UserWidget.AddToViewport` _returnvalue 0)))
    (:`then_1`
      (if (== (`self.eggs`) 5)
        (`KismetSystemLibrary.Delay` 1.0)
        (set `self.Seconds` (- (`self.Seconds`) 1))
        (if (< (`self.Seconds`) 0)
          (set `self.Minutes` (- (`self.Minutes`) 1))
          (set `self.Seconds` 59))
        (if (== (`self.Seconds`) 0)
          (if (== (`self.Minutes`) 0)
            (`/Engine/EditorBlueprintResources/StandardMacros.DoOnce` false
              (:`Completed`
                (`KismetSystemLibrary.PrintString` "GameOver")))))))))

(fn `UserConstructionScript`)