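; BP_Nest is a nest actor that collects eggs carried by the player and loses health while under attack.
; An EggSphere overlap deposits the player's carried egg, raising nest and GameMode counts, and Tick reveals the matching one of five initially hidden egg components.
; Any overlap with Sphere flags an attack, and a Delay on Tick paces repeated damage.
; Tick mirrors health to BP_GameMode; destruction only prints a message.
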(event `self.ReceiveTick`
  (params (DeltaSeconds :type "Float (single-precision)"))
  (`|ExecutionSequence`
    (:`then_0`
      (if (== (`self.Eggs`) 1)
        (`SceneComponent.SetHiddenInGame` (`self.Egg1`) false false)))
    (:`then_1`
      (if (== (`self.Eggs`) 2)
        (`SceneComponent.SetHiddenInGame` (`self.Egg2`) false false)))
    (:`then_2`
      (if (== (`self.Eggs`) 3)
        (`SceneComponent.SetHiddenInGame` (`self.Egg3`) false false)))
    (:`then_3`
      (if (== (`self.Eggs`) 4)
        (`SceneComponent.SetHiddenInGame` (`self.Egg4`) false false)))
    (:`then_4`
      (if (== (`self.Eggs`) 5)
        (`SceneComponent.SetHiddenInGame` (`self.Egg5`) false false)))
    (:`then_5`
      (if (<= (`self.Health`) 0.0)
        (`/Engine/EditorBlueprintResources/StandardMacros.DoOnce` false
          (:`Completed`
            (`KismetSystemLibrary.PrintString` "NestDestroyed")))))
    (:`then_6`
      (bind _asbp_game_mode (cast `/Game/Blueprints/BP_GameMode` (`GameplayStatics.GetGameMode`)))
      (set `/Game/Blueprints/BP_GameMode.NestHealth` (`self.Health`) _asbp_game_mode))
    (:`then_7`
      (if (`self.IsAttacked`)
        (`KismetSystemLibrary.Delay` 1.0)
        (`self.Damage`)))))

(event `self.EggSphere.OnComponentBeginOverlap`
  (params (OverlappedComponent :type "PrimitiveComponent Object Reference") (OtherActor :type "Actor Object Reference") (OtherComp :type "PrimitiveComponent Object Reference") (OtherBodyIndex :type Integer) (bFromSweep :type Boolean) (SweepResult :type "HitResult Structure (by ref)"))
  (bind _asbp_character (cast `/Game/Blueprints/BP_Character` (`GameplayStatics.GetPlayerPawn` 0)))
  (if (`/Game/Blueprints/BP_Character.EggPickedUp` _asbp_character)
    (set `self.Eggs` (+ (`self.Eggs`) 1))
    (set `/Game/Blueprints/BP_Character.EggPickedUp` false _asbp_character)
    (bind _asbp_game_mode (cast `/Game/Blueprints/BP_GameMode` (`GameplayStatics.GetGameMode`)))
    (set `/Game/Blueprints/BP_GameMode.eggs` (+ (`/Game/Blueprints/BP_GameMode.eggs` _asbp_game_mode) 1) _asbp_game_mode)))

(event `self.Sphere.OnComponentBeginOverlap`
  (params (OverlappedComponent :type "PrimitiveComponent Object Reference") (OtherActor :type "Actor Object Reference") (OtherComp :type "PrimitiveComponent Object Reference") (OtherBodyIndex :type Integer) (bFromSweep :type Boolean) (SweepResult :type "HitResult Structure (by ref)"))
  (set `self.IsAttacked` true))

(event `self.Sphere.OnComponentEndOverlap`
  (params (OverlappedComponent :type "PrimitiveComponent Object Reference") (OtherActor :type "Actor Object Reference") (OtherComp :type "PrimitiveComponent Object Reference") (OtherBodyIndex :type Integer))
  (set `self.IsAttacked` false))

(event `self.ReceiveBeginPlay`
  ;[1 1 1] Set all eggs Hidden
  (`SceneComponent.SetHiddenInGame` (`self.Egg1`) true false)
  (`SceneComponent.SetHiddenInGame` (`self.Egg2`) true false)
  (`SceneComponent.SetHiddenInGame` (`self.Egg5`) true false)
  (`SceneComponent.SetHiddenInGame` (`self.Egg4`) true false)
  (`SceneComponent.SetHiddenInGame` (`self.Egg3`) true false))

(event `Damage`
  ;[1 1 1] damage
  (`KismetSystemLibrary.PrintString` "NestHit")
  (set `self.Health` (- (`self.Health`) 5.0)))

(fn `UserConstructionScript`)