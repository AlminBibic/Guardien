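; BP_Egg is a pickup egg that hovers and spins in the level.
; Any Sphere overlap checks the player pawn as BP_Character, whatever actor overlapped; if EggPickedUp is false, it sets it and destroys the egg.
; A Hover timeline started on BeginPlay adds half its value to the current Z each update, so offsets accumulate.
; Tick adds a fixed yaw step per frame, making spin speed frame-rate dependent.
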(event `self.Sphere.OnComponentBeginOverlap`
  (params (OverlappedComponent :type "PrimitiveComponent Object Reference") (OtherActor :type "Actor Object Reference") (OtherComp :type "PrimitiveComponent Object Reference") (OtherBodyIndex :type Integer) (bFromSweep :type Boolean) (SweepResult :type "HitResult Structure (by ref)"))
  (bind _asbp_character (cast `/Game/Blueprints/BP_Character` (`GameplayStatics.GetPlayerPawn` 0)))
  (if (not (`/Game/Blueprints/BP_Character.EggPickedUp` _asbp_character))
    (set `/Game/Blueprints/BP_Character.EggPickedUp` true _asbp_character)
    (`self.K2_DestroyActor`)))

(event `self.ReceiveBeginPlay`
  (bind (_returnvalue_x _returnvalue_y _returnvalue_z) (`KismetMathLibrary.BreakVector` (`self.K2_GetActorLocation`)))
  ;[1 1 1] Object Hover
  (bind (_direction _hover) (`Timeline|Hover`)
    (:`Update`
      (`self.K2_SetActorLocation` (`KismetMathLibrary.MakeVector` _returnvalue_x _returnvalue_y (+ _returnvalue_z (/ _hover 2.0)))))))

(event `self.ReceiveTick`
  (params (DeltaSeconds :type "Float (single-precision)"))
  (bind (_returnvalue_roll _returnvalue_pitch _returnvalue_yaw) (`KismetMathLibrary.BreakRotator` (`self.K2_GetActorRotation`)))
  ;[1 1 1] Object Hover
  (`self.K2_SetActorRotation` (`KismetMathLibrary.MakeRotator` _returnvalue_roll _returnvalue_pitch (+ _returnvalue_yaw 1.0))))

(fn `UserConstructionScript`)