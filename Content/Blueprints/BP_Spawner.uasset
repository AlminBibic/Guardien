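; BP_Spawner is an actor that spawns BP_Enemy instances once the BP_GameMode Start flag is set.
; Tick spawns an enemy at the Sphere component's transform until CurrentSpawn equals MaxSpawn, always spawning despite collisions.
; Each enemy receives TargetPoint as its Target and CrocoRotation as its NewRotation.
; The trailing SpawnDelay Delay has nothing after it, so spawns occur on consecutive ticks.
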(event `self.ReceiveTick`
  (params (DeltaSeconds :type "Float (single-precision)"))
  (bind _asbp_game_mode (cast `/Game/Blueprints/BP_GameMode` (`GameplayStatics.GetGameMode`)))
  (if (`/Game/Blueprints/BP_GameMode.Start` _asbp_game_mode)
    (if (not (== (`self.CurrentSpawn`) (`self.MaxSpawn`)))
      (bind _returnvalue (`|SpawnActorFromClass` "/Game/Blueprints/BP_Enemy.BP_Enemy_C" (`SceneComponent.K2_GetComponentToWorld` (`self.Sphere`)) "AlwaysSpawn" "OverrideRootScale" null null))
      (set `/Game/Blueprints/BP_Enemy.Target` (`self.TargetPoint`) _returnvalue)
      (set `PEnemy.NewRotation` (`self.CrocoRotation`) _returnvalue)
      (set `self.CurrentSpawn` (+ (`self.CurrentSpawn`) 1))
      (`KismetSystemLibrary.Delay` (`self.SpawnDelay`)))))

(fn `UserConstructionScript`)